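; Environment spawner that streams endless level segments along the X axis around the first BP_ThirdPersonCharacter found.
; BeginPlay spawns each EnviroBP class once in a row, advancing the spawn point by a fixed segment length.
; Tick destroys segments far behind the player and appends random ones while the spawn point is within a set range ahead.
; DeleteFarActors duplicates the cleanup with a debug print but is not called here.
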(event EventBeginPlay
  (bind _outactors (Actor|GetAllActorsOfClass "/Game/ThirdPerson/Blueprints/BP_ThirdPersonCharacter.BP_ThirdPersonCharacter_C"))
  (bind _output_get (Variables|Default|SetBP_ThirdPerson _outactors))
  (Variables|Default|SetPlayerCharacter (Utilities|Array|Get(acopy) _output_get))
  (for _array_element (Variables|Default|GetEnviroBP)
    (bind _returnvalue (Game|SpawnActorfromClass _array_element (Math|Transform|MakeTransform (Variables|Default|GetSpawnEnvironmentLocation) "0, 0, 0" "1.000000,1.000000,1.000000") "Undefined" "MultiplyWithRoot" 0 0))
    (Utilities|Array|Add (Variables|Default|GetSpawnedEnvironment) _returnvalue)
    (Variables|Default|SetSpawnEnvironmentLocation (Math|Vector|MakeVector (+ (.x (Variables|Default|GetSpawnEnvironmentLocation)) 1e+04) (.y (Variables|Default|GetSpawnEnvironmentLocation)) (.z (Variables|Default|GetSpawnEnvironmentLocation))))))

(event EventTick
  (params (DeltaSeconds :type Float%20%28single-precision%29))
  (bind _playercharacter (Variables|Default|GetPlayerCharacter))
  (bind _playercharacter_2 (Variables|Default|GetPlayerCharacter))
  ;[0.4455 1 0.9502] Checks if the actor should be deleted
  (for (_array_element _array_index) (Variables|Default|GetSpawnedEnvironment)
    (Utilities|IsValid _playercharacter_2
      (:Is%20Valid
        (bind _output_get (Variables|Default|SetEnviroTemp _array_element))
        (if (> (- (.x (.location (Transformation|GetWorldTransform (Variables|/Script/Engine.Actor|GetRootComponent _playercharacter_2)))) (.x (.location (Transformation|GetWorldTransform (Variables|/Script/Engine.Actor|GetRootComponent _output_get))))) 2e+04)
          (Utilities|Array|RemoveIndex (Variables|Default|GetSpawnedEnvironment) _array_index)
          (Actor|DestroyActor (Variables|Default|GetEnviroTemp))))))
  ;[1 1 1] if spawn is less than 3 units spawn
  (if (Utilities|IsValid _playercharacter)
    (if (and (< (- (.x (.location (Transformation|GetActorTransform _playercharacter))) (.x (Variables|Default|GetSpawnEnvironmentLocation))) -1e+04) (> (- (.x (.location (Transformation|GetActorTransform _playercharacter))) (.x (Variables|Default|GetSpawnEnvironmentLocation))) -5e+04))
      ;[1 1 1] Choose a random environment to spawn
      (bind _returnvalue (Game|SpawnActorfromClass (.OutItem (Utilities|Array|Random (Variables|Default|GetEnviroBP))) (Math|Transform|MakeTransform (Variables|Default|GetSpawnEnvironmentLocation) "0, 0, 0" "1.000000,1.000000,1.000000") "Undefined" "MultiplyWithRoot" 0 0))
      (Utilities|Array|Add (Variables|Default|GetSpawnedEnvironment) _returnvalue)
      (Variables|Default|SetSpawnEnvironmentLocation (Math|Vector|MakeVector (+ (.x (Variables|Default|GetSpawnEnvironmentLocation)) 1e+04) (.y (Variables|Default|GetSpawnEnvironmentLocation)) (.z (Variables|Default|GetSpawnEnvironmentLocation)))))))

(fn ConstructionScript)

(fn DeleteFarActors
  (for (_array_element _array_index) (Variables|Default|GetSpawnedEnvironment)
    (if (> (- (.x (.location (Transformation|GetWorldTransform (Variables|/Script/Engine.Actor|GetRootComponent (Variables|Default|GetPlayerCharacter))))) (.x (.location (Transformation|GetWorldTransform (Variables|/Script/Engine.Actor|GetRootComponent _array_element))))) 2e+04)
      (Utilities|Array|RemoveIndex (Variables|Default|GetSpawnedEnvironment) _array_index)
      (Actor|DestroyActor _array_element)
      (Development|PrintString "deleted something")))
  (return false))