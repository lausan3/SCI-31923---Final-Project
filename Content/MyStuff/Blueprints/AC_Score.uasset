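; AC_Score is a score component that tracks the player pawn's Y progress from its spawn point and detects when it stops moving.
; Each AddScore call adds the current Y offset from the start to the score, saves the position and flags movement as started.
; Once started, Tick calls GameOver whenever the pawn's position exactly matches that saved position; GameOver only prints a message.
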(event Custom|AddScore
  (bind _returnvalue (Game|Player|GetPlayerPawn 0))
  (bind _returnvalue_2 (Transformation|GetActorTransform _returnvalue))
  (bind _returnvalue_3 (Math|Transform|TransformLocation _returnvalue_2 "0, 0, 0"))
  ;[1 1 1] Func AddScore - adds difference of current Y and starting Y to score float
  (Variables|Default|SetScore (+ (Variables|Default|GetScore) (- (.Y (Math|Vector|BreakVector _returnvalue_3)) (.Y (Math|Vector|BreakVector (Variables|Default|GetStartingVector))))))
  (Variables|Default|SetLastMovementVector _returnvalue_3)
  (if (not (Variables|Default|GetStartedMoving))
    (Variables|Default|SetStartedMoving true)))

(event Custom|GameOver
  (Development|PrintString "u stopped moving dummy"))

(event EventBeginPlay
  ;[1 1 1] Event Begin Play - set starting Y to Y at player spawn point
  (Variables|Default|SetStartingVector (Math|Transform|TransformLocation (Transformation|GetActorTransform (Game|Player|GetPlayerPawn 0)) "0, 0, 0")))

(event EventTick
  (params (DeltaSeconds :type Float%20%28single-precision%29))
  ;[1 1 1] Event Tick - if we've started moving and we stop, call GameOver event
  (if (Variables|Default|GetStartedMoving)
    (if (Utilities|Operators|EqualEqual (Variables|Default|GetLastMovementVector) (Math|Transform|TransformLocation (Transformation|GetActorTransform (Game|Player|GetPlayerPawn 0)) "0, 0, 0") 0.0)
      (CallFunction|GameOver))))