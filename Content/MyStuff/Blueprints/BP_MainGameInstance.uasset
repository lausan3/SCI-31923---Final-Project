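; BP_MainGameInstance is a Game Instance Blueprint that holds the game's score, game-over flag and player health.
; Custom events set the game-over flag and store incoming score divided by ten.
; Health events add a given amount, apply passive healing scaled by tick delta toward a full heal over a configured duration, or reset to maximum.
; Both additive health events clamp the result between zero and max health.
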(event Custom|UpdateScore
  (params (NewScore :type Float%20%28double-precision%29))
  ;[1 1 1] Update Score (float NewScore)
  (Variables|Default|SetScore (/ NewScore 1e+01)))

(event Custom|SetGameOver
  (params (newGameOver :type Boolean))
  ;[1 1 1] Set Game Over (bool NewGameOver)
  (Variables|Default|SetisGameOver newGameOver))

(event Custom|ResetPlayerHealth
  ;[1 1 1] Reset Player Health
  (Variables|Default|SetPlayerHealth (Variables|Default|GetMaxHealth)))

(event Custom|AddPlayerHealth
  (params (HealthToAdd :type Float%20%28double-precision%29))
  ;[1 1 1] Add Player Health (float HealthToAdd)
  (Variables|Default|SetPlayerHealth (Math|Float|Clamp(Float) (+ HealthToAdd (Variables|Default|GetPlayerHealth)) 0.0 (Variables|Default|GetMaxHealth))))

(event Custom|AddPassiveHealing
  (params (Tick%20Delta :type Float%20%28double-precision%29))
  ;[1 1 1] Add Passive Healing (float TickDelta)
  (Variables|Default|SetPlayerHealth (Math|Float|Clamp(Float) (+ (Variables|Default|GetPlayerHealth) (* (/ Tick%20Delta (Variables|Default|GetSecsToFullHeal)) (Variables|Default|GetMaxHealth))) 0.0 (Variables|Default|GetMaxHealth))))